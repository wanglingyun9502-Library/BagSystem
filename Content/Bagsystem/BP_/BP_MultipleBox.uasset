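; BP_MultipleBox is a container actor in the bag system that shows its contents in the player's box UI when approached.
; Sphere overlap by the player character sets IsCollisionBox and passes RemoveArray to CreateuiPawn.
; Any end overlap, without an actor check, resets the flag and clears BoxUI.
; RemoveDragObject removes a given entry from RemoveArray; a debug print loop is left unconnected.
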(event OnComponentBeginOverlap(Sphere)
  (params (OverlappedComponent :type Primitive%20Component%20Object%20Reference) (OtherActor :type Actor%20Object%20Reference) (OtherComp :type Primitive%20Component%20Object%20Reference) (OtherBodyIndex :type Integer) (bFromSweep :type Boolean) (SweepResult :type Hit%20Result%20Structure%20%28by%20ref%29))
  (bind _playpawn (Variables|Default|GetPlaypawn))
  ;[1 1 1] Comment
  (if (== _playpawn OtherActor)
    (Variables|/Game/ThirdPersonBP/Blueprints/ThirdPersonCharacter.ThirdPersonCharacter_C|SetIsCollisionBox? _playpawn true)
    (Default|CreateuiPawn (Variables|Default|GetPlaypawn) (Variables|Default|GetRemoveArray))))

(event OnComponentEndOverlap(Sphere)
  (params (OverlappedComponent :type Primitive%20Component%20Object%20Reference) (OtherActor :type Actor%20Object%20Reference) (OtherComp :type Primitive%20Component%20Object%20Reference) (OtherBodyIndex :type Integer))
  ;[1 1 1] Comment
  (Variables|/Game/ThirdPersonBP/Blueprints/ThirdPersonCharacter.ThirdPersonCharacter_C|SetIsCollisionBox? (Variables|Default|GetPlaypawn) false)
  (Default|CleraUI (Variables|/Game/Bagsystem/Widget/Main_UI.Main_UI_C|GetBoxUI (Variables|/Game/ThirdPersonBP/Blueprints/ThirdPersonCharacter.ThirdPersonCharacter_C|GetMainUI (Variables|Default|GetPlaypawn)))))

(event EventBeginPlay
  (bind _returnvalue (Game|GetPlayerCharacter 0))
  ;[1 1 1] Comment
  (if (Utilities|IsValid _returnvalue)
    (bind _asthird_person_character (Utilities|Casting|CastToThirdPersonCharacter _returnvalue))
    (Variables|Default|SetPlaypawn _asthird_person_character)))

(fn ConstructionScript)

(fn RemoveDragObject
  (params (RemoveObj :type String%20%28by%20ref%29))
  (Utilities|Array|RemoveItem (Variables|Default|GetRemoveArray) RemoveObj))