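; BP_SingleObject is a pickup item in the bag system that the player collects with the PickActor input while inside its sphere.
; The construction script sets the mesh and derives name and type from the mesh name's prefix, building InfoStruct before assigning the type.
; Overlap creates pickup UI on ThirdPersonCharacter; ending it briefly toggles sphere collision.
; Pickup adds the item to the bag, then hides it, disables collision and moves it to origin.
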(event OnComponentBeginOverlap(Sphere)
  (params (OverlappedComponent :type Primitive%20Component%20Object%20Reference) (OtherActor :type Actor%20Object%20Reference) (OtherComp :type Primitive%20Component%20Object%20Reference) (OtherBodyIndex :type Integer) (bFromSweep :type Boolean) (SweepResult :type Hit%20Result%20Structure%20%28by%20ref%29))
  (bind _third_person_character (Variables|Game|GetThird%20Person%20Character))
  (if (== (Variables|Game|GetThird%20Person%20Character) OtherActor)
    ;[1 1 1] 获取actor名称，自动生成UI 用
    (Variables|Game|SetIsplayerOverlap? true)
    (Variables|/Game/ThirdPersonBP/Blueprints/ThirdPersonCharacter.ThirdPersonCharacter_C|SetIsCollisionBox? _third_person_character true)
    (Variables|Default|SetRechick true)
    (Default|CreateuiPawn _third_person_character "NewEnumerator0" (Utilities|Array|MakeArray (Variables|ActorInfo|GetInfoStruct)))
    (Development|PrintString "ininin")))

(event OnComponentEndOverlap(Sphere)
  (params (OverlappedComponent :type Primitive%20Component%20Object%20Reference) (OtherActor :type Actor%20Object%20Reference) (OtherComp :type Primitive%20Component%20Object%20Reference) (OtherBodyIndex :type Integer))
  (bind _sphere (Variables|Default|GetSphere))
  (Variables|Game|SetIsplayerOverlap? false)
  (Default|MovePawn (Variables|Game|GetThird%20Person%20Character))
  (Collision|SetCollisionEnabled _sphere "NoCollision")
  (Utilities|FlowControl|Delay 0.01)
  (Collision|SetCollisionEnabled _sphere "QueryAndPhysics"))

(event EventBeginPlay
  (bind _asthird_person_character (Utilities|Casting|CastToThirdPersonCharacter (Game|Player|GetPlayerPawn 0)))
  (Variables|Game|SetThird%20Person%20Character _asthird_person_character))

(event EventTick
  (params (DeltaSeconds :type Float%20%28single-precision%29)))

(event Input|ActionEvents|InputActionPickActor
  (params (Key :type Key%20Structure :default "None"))
  ;[1 1 1] 拾取武器之后的操作
  (:Pressed
    (if (Variables|Game|GetIsplayerOverlap?)
      (Default|JoinPlayerBag (Variables|Game|GetThird%20Person%20Character) (Utilities|Struct|MakeSinlegResourceStruct (Variables|ActorInfo|GetName) self (Variables|ActorInfo|GetActor%20Type) (Variables|ActorInfo|GetActor%20Image)))
      (CallFunction|Pickactor)))
  (:Released
    (Default|Updataremove (Variables|/Game/Bagsystem/Widget/Main_UI.Main_UI_C|GetBoxUI (Variables|/Game/ThirdPersonBP/Blueprints/ThirdPersonCharacter.ThirdPersonCharacter_C|GetMainUI (Variables|Game|GetThird%20Person%20Character))))))

(fn ConstructionScript
  (bind _weaponactor (Variables|Default|GetWeaponActor))
  (bind _weaponmesh (Variables|Game|GetWeaponmesh))
  (bind _returnvalue (Utilities|GetObjectName _weaponmesh))
  (Components|StaticMesh|SetStaticMesh _weaponactor _weaponmesh)
  (Transformation|SetRelativeRotation _weaponactor "0, 0,90.000000" false false)
  (bind _output_get (Variables|ActorInfo|SetName _returnvalue))
  (Variables|ActorInfo|SetInfoStruct (Utilities|Struct|MakeSinlegResourceStruct _output_get self (Variables|ActorInfo|GetActor%20Type) (Variables|ActorInfo|GetActor%20Image)))
  (switch string (.LeftS (Utilities|String|Split _returnvalue "_"))
    (:Wp
      (Variables|ActorInfo|SetActor%20Type "NewEnumerator0"))
    (:Dr
      (Variables|ActorInfo|SetActor%20Type "NewEnumerator6"))))

(fn Pickactor
  (Rendering|SetActorHiddenInGame true)
  (Collision|SetCollisionEnabled (Variables|Default|GetSphere) "NoCollision")
  (Transformation|SetActorLocation "0, 0, 0" false false)
  (Variables|/Game/ThirdPersonBP/Blueprints/ThirdPersonCharacter.ThirdPersonCharacter_C|SetIsCollisionBox? (Variables|Game|GetThird%20Person%20Character) true))