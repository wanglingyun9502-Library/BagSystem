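; Single pickup item for the bag system, building its mesh and equip info struct in the construction script.
; Sphere overlap shows nearby-item UI on ThirdPersonCharacter; PickActor adds it to the bag and destroys it, provided IsPick is set.
; Tick clears IsPick and custom-depth highlight during overlap, so both need external refreshing.
; End overlap and CastoffFuction (drop) toggle sphere collision to re-detect overlaps.
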(event OnComponentBeginOverlap(Sphere)
  (params (OverlappedComponent :type Primitive%20Component%20Object%20Reference) (OtherActor :type Actor%20Object%20Reference) (OtherComp :type Primitive%20Component%20Object%20Reference) (OtherBodyIndex :type Integer) (bFromSweep :type Boolean) (SweepResult :type Hit%20Result%20Structure%20%28by%20ref%29))
  ;[1 1 1] 进入碰撞，获取actor名称，自动生成UI 用
  (if (== (Variables|Game|GetThird%20Person%20Character) OtherActor)
    (Variables|Game|SetIsplayerOverlap? true)
    (Variables|Game|SetRechick true)
    (Default|CreateuiPawn (Variables|Game|GetThird%20Person%20Character) "NewEnumerator0" (Variables|ActorInfo|GetInfoStruct))
    (Variables|/Game/ThirdPersonBP/Blueprints/ThirdPersonCharacter.ThirdPersonCharacter_C|SetIsCollisionBox? (Variables|Game|GetThird%20Person%20Character) true)))

(event OnComponentEndOverlap(Sphere)
  (params (OverlappedComponent :type Primitive%20Component%20Object%20Reference) (OtherActor :type Actor%20Object%20Reference) (OtherComp :type Primitive%20Component%20Object%20Reference) (OtherBodyIndex :type Integer))
  (bind _sphere (Variables|Default|GetSphere))
  (bind _third_person_character (Variables|Game|GetThird%20Person%20Character))
  ;[1 1 1] 出碰撞
  (Variables|Game|SetIsplayerOverlap? false)
  (Variables|/Game/ThirdPersonBP/Blueprints/ThirdPersonCharacter.ThirdPersonCharacter_C|SetIsCollisionBox? _third_person_character false)
  (Default|CleraWidget (Variables|/Game/Bagsystem/Widget/BP_Main_Widget.BP_Main_Widget_C|GetBP_NearResource_Widget_58 (Variables|/Game/ThirdPersonBP/Blueprints/ThirdPersonCharacter.ThirdPersonCharacter_C|Getbp_Main_ui _third_person_character)))
  ;[1 1 1] 当出碰撞时，先让物体的碰撞消失，然后在显示，这样可以解决一个物体消失之后，人物还在另一个碰撞中，但是无法识别的情况
  (Collision|SetCollisionEnabled _sphere "NoCollision")
  (Utilities|FlowControl|Delay 0.001)
  (Collision|SetCollisionEnabled _sphere "QueryAndPhysics"))

(event Custom|CheckCollision
  (bind _sphere (Variables|Default|GetSphere))
  ;[1 1 1] 当出碰撞时，先让物体的碰撞消失，然后在显示，这样可以解决一个物体消失之后，人物还在另一个碰撞中，但是无法识别的情况
  (Collision|SetCollisionEnabled _sphere "NoCollision")
  (Utilities|FlowControl|Delay 0.001)
  (Collision|SetCollisionEnabled _sphere "QueryAndPhysics"))

(event Custom|UnActive%20Mesh%20Custom%20Depth
  ;[1 1 1] 设置高亮
  (Rendering|SetRenderCustomDepth (Variables|Default|GetWeaponActor) false))

(event Custom|Active%20Mesh%20Custom%20Depth
  ;[1 1 1] 设置高亮
  (if (Variables|Game|GetIsplayerOverlap?)
    (Rendering|SetRenderCustomDepth (Variables|Default|GetWeaponActor) true)))

(event EventBeginPlay
  (bind _asthird_person_character (Utilities|Casting|CastToThirdPersonCharacter (Game|Player|GetPlayerPawn 0)))
  (Variables|Game|SetThird%20Person%20Character _asthird_person_character))

(event EventTick
  (params (DeltaSeconds :type Float%20%28single-precision%29))
  (if (Variables|Game|GetIsplayerOverlap?)
    (CallFunction|UnActiveMeshCustomDepth)
    (Variables|Game|SetIsPick false)))

(event Input|ActionEvents|InputActionPickActor
  (params (Key :type Key%20Structure :default "None"))
  ;[1 1 1] 拾取武器之后的操作（按下F）
  (:Pressed
    (if (Variables|Game|GetIsplayerOverlap?)
      (if (Variables|Game|GetIsPick)
        (Default|JoinPlayerBag (Variables|Game|GetThird%20Person%20Character) (Variables|ActorInfo|GetInfoStruct))
        (CallFunction|DestoryEquip)))))

(fn ConstructionScript
  (bind _weaponactor (Variables|Default|GetWeaponActor))
  (Components|StaticMesh|SetStaticMesh _weaponactor (Variables|Game|GetWeaponmesh))
  (Transformation|SetRelativeRotation _weaponactor "0, 0,90.000000" false false)
  (Variables|ActorInfo|SetInfoStruct (Utilities|Struct|MakeEuqipInfoStruct (Variables|ActorInfo|GetActorInfo) self (Variables|ActorInfo|GetActor%20Type) (Variables|ActorInfo|GetActor%20Image) (Variables|ActorInfo|GetNumber) (Variables|Game|GetWeaponmesh))))

(fn DestoryEquip
  (Rendering|SetActorHiddenInGame true)
  (Collision|SetCollisionEnabled (Variables|Default|GetSphere) "NoCollision")
  (Transformation|SetActorLocation "0, 0,-10.000000" false false)
  (Actor|DestroyActor))

(fn CastoffFuction
  (params (Castoff_Location :type Vector) (Castoff_Rotation :type Rotator))
  (bind _sphere (Variables|Default|GetSphere))
  (Rendering|SetActorHiddenInGame false)
  (Collision|SetCollisionEnabled (Variables|Default|GetSphere) "QueryAndPhysics")
  (Transformation|SetActorLocation Castoff_Location false false)
  (Transformation|SetActorRotation Castoff_Rotation)
  (Collision|SetCollisionEnabled _sphere "NoCollision")
  (Collision|SetCollisionEnabled _sphere "QueryAndPhysics")
  (CallFunction|CheckCollision))