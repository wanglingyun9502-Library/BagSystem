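; BP_MultipleBox is a multi-item box for the bag system, holding its contents in RemoveArray.
; BeginPlay caches the player's ThirdPersonCharacter as Playpawn.
; RemoveDragObject removes entries matching a given name from the array after an item is dragged out of the box.
; The Sphere overlap events are empty, with disconnected logic for setting the player's collision flag and creating or clearing the box UI.
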(event OnComponentBeginOverlap(Sphere)
  (params (OverlappedComponent :type Primitive%20Component%20Object%20Reference) (OtherActor :type Actor%20Object%20Reference) (OtherComp :type Primitive%20Component%20Object%20Reference) (OtherBodyIndex :type Integer) (bFromSweep :type Boolean) (SweepResult :type Hit%20Result%20Structure%20%28by%20ref%29))
  ;[1 1 1] Comment
)

(event OnComponentEndOverlap(Sphere)
  (params (OverlappedComponent :type Primitive%20Component%20Object%20Reference) (OtherActor :type Actor%20Object%20Reference) (OtherComp :type Primitive%20Component%20Object%20Reference) (OtherBodyIndex :type Integer))
  ;[1 1 1] Comment
)

(event EventBeginPlay
  (bind _returnvalue (Game|GetPlayerCharacter 0))
  ;[1 1 1] Comment
  (if (Utilities|IsValid _returnvalue)
    (bind _asthird_person_character (Utilities|Casting|CastToThirdPersonCharacter _returnvalue))
    (Variables|Default|SetPlaypawn _asthird_person_character)))

(fn ConstructionScript)

(fn RemoveDragObject
  (params (RemoveObj :type String%20%28by%20ref%29))
  ;[1 1 1] 盒子中每次拖拽完成之后，清除盒子中物体的数组中的拖拽完成的元素
  (for _array_element (Variables|Default|GetRemoveArray)
    (if (Utilities|Enum|Equal(Enum) RemoveObj (.Name (Utilities|Struct|BreakEuqipInfoStruct _array_element)))
      (Utilities|Array|RemoveItem :TargetArray (Variables|Default|GetRemoveArray)))))